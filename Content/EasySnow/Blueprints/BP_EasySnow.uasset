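; Snow weather actor that drives a Niagara snowfall and drifting-snow effect, plus snow settings for world materials.
; The construction script builds dynamic flake, sprite and drift materials (or debug versions per distance band) and pushes exposed settings to Niagara.
; A valid Preset overrides the main particle values and copies them back into the actor's variables.
; Tick republishes wind and optional world-snow parameters to the MP_WF_WorldData collection and updates simulation speed.
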(event Collision|EventActorBeginOverlap
  (params (OtherActor :type Actor%20Object%20Reference)))

(event EventTick
  (params (DeltaSeconds :type Float%20%28single-precision%29))
  (Rendering|Material|SetScalarParameterValue "/Game/EasySnow/System/MP_WF_WorldData.MP_WF_WorldData" "windDirection" (Variables|EasySnowSettings|Wind|GetwindDirection) :!class /Script/Engine.KismetMaterialLibrary)
  (Rendering|Material|SetScalarParameterValue "/Game/EasySnow/System/MP_WF_WorldData.MP_WF_WorldData" "windStrength" (Variables|EasySnowSettings|Wind|GetwindStrength%20-) :!class /Script/Engine.KismetMaterialLibrary)
  (Rendering|Material|SetScalarParameterValue "/Game/EasySnow/System/MP_WF_WorldData.MP_WF_WorldData" "windBuildupOverride" (Variables|EasySnowSettings|WorldMaterialSettings|GetwindBuildupOverride) :!class /Script/Engine.KismetMaterialLibrary)
  (Class|NiagaraComponent|SetCustomTimeDilation (Variables|Default|GetSnowBP) (Variables|EasySnowSettings|GetcustomSpeed%20-))
  (if (Variables|EasySnowSettings|WorldMaterialSettings|GetSet%20World%20Snow%20Material%20Settings)
    (Rendering|Material|SetScalarParameterValue "/Game/EasySnow/System/MP_WF_WorldData.MP_WF_WorldData" "Snow Glimmering Intensity" (Variables|EasySnowSettings|WorldMaterialSettings|GetSnow%20Glimmer%20Intensity) :!class /Script/Engine.KismetMaterialLibrary)
    (Rendering|Material|SetScalarParameterValue "/Game/EasySnow/System/MP_WF_WorldData.MP_WF_WorldData" "Snow Displacement Multiplier" (Variables|EasySnowSettings|WorldMaterialSettings|GetWorld%20Snow%20Displacement%20Multiplier) :!class /Script/Engine.KismetMaterialLibrary)
    (Rendering|Material|SetScalarParameterValue "/Game/EasySnow/System/MP_WF_WorldData.MP_WF_WorldData" "Z Offset" (Variables|EasySnowSettings|WorldMaterialSettings|GetZ%20%20Offset) :!class /Script/Engine.KismetMaterialLibrary)
    (Rendering|Material|SetScalarParameterValue "/Game/EasySnow/System/MP_WF_WorldData.MP_WF_WorldData" "Transition Sharpness" (Variables|EasySnowSettings|WorldMaterialSettings|GetTransition%20Sharpness) :!class /Script/Engine.KismetMaterialLibrary)
    (Rendering|Material|SetScalarParameterValue "/Game/EasySnow/System/MP_WF_WorldData.MP_WF_WorldData" "Breakup Intensity" (Variables|EasySnowSettings|WorldMaterialSettings|GetbreakupIntensity) :!class /Script/Engine.KismetMaterialLibrary)
    (Rendering|Material|SetScalarParameterValue "/Game/EasySnow/System/MP_WF_WorldData.MP_WF_WorldData" "Breakup Texture Tiling" (Math|Conversions|ToFloat(Integer) (Class|KismetMathLibrary|ToInt64(Float) (Variables|EasySnowSettings|WorldMaterialSettings|GetbreakupTextureTiling))) :!class /Script/Engine.KismetMaterialLibrary)
    (Rendering|Material|SetScalarParameterValue "/Game/EasySnow/System/MP_WF_WorldData.MP_WF_WorldData" "Snow Fade Control" (Variables|EasySnowSettings|WorldMaterialSettings|GetsnowFadeControl) :!class /Script/Engine.KismetMaterialLibrary)
    (Rendering|Material|SetScalarParameterValue "/Game/EasySnow/System/MP_WF_WorldData.MP_WF_WorldData" "Snow Amount" (Variables|EasySnowSettings|WorldMaterialSettings|GetsnowAmount) :!class /Script/Engine.KismetMaterialLibrary)))

(fn ConstructionScript
  (bind _snowbp (Variables|Default|GetSnowBP))
  (bind _snowbp_2 (Variables|Default|GetSnowBP))
  (bind _snowbp_3 (Variables|Default|GetSnowBP))
  (bind _debugtoggle (Variables|EasySnowSettings|LODControl|GetDebugToggle))
  (bind _snowbp_4 (Variables|Default|GetSnowBP))
  (bind _snowbp_5 (Variables|Default|GetSnowBP))
  (bind _snowbp_6 (Variables|Default|GetSnowBP))
  (bind _snowbp_7 (Variables|Default|GetSnowBP))
  (bind _snowbp_8 (Variables|Default|GetSnowBP))
  (bind _snowbp_9 (Variables|Default|GetSnowBP))
  (bind _snowbp_10 (Variables|Default|GetSnowBP))
  (bind _snowbp_11 (Variables|Default|GetSnowBP))
  (bind _snowbp_12 (Variables|Default|GetSnowBP))
  (bind _snowbp_13 (Variables|Default|GetSnowBP))
  (bind _snowbp_14 (Variables|Default|GetSnowBP))
  (bind _snowbp_15 (Variables|Default|GetSnowBP))
  (bind _snowbp_16 (Variables|Default|GetSnowBP))
  (bind _snowbp_17 (Variables|Default|GetSnowBP))
  (bind _returnvalue (Math|Conversions|ToFloat(Boolean) _debugtoggle))
  (if (Variables|EasySnowSettings|LODControl|GetDebugToggle)
    ;[0.7841 0.2067 1] DEBUGGING
    (bind _returnvalue_2 (Rendering|Material|CreateDynamicMaterialInstance "/Game/EasySnow/Materials/Masters/M_niagaraSnow.M_niagaraSnow" "None" "None" :!class /Script/Engine.KismetMaterialLibrary))
    (bind _output_get (Variables|EasySnowSettings|SetDynamicMaterial _returnvalue_2))
    (Class|NiagaraComponent|SetVariableMaterial (Variables|Default|GetSnowBP) "NiagaraDebug_Near" _output_get)
    (Rendering|Material|SetScalarParameterValue (Variables|EasySnowSettings|GetDynamicMaterial) "DebugToggleMaterial_Near" _returnvalue :!class /Script/Engine.MaterialInstanceDynamic)
    (bind _returnvalue_3 (Rendering|Material|CreateDynamicMaterialInstance "/Game/EasySnow/Materials/Masters/M_niagaraSnow.M_niagaraSnow" "None" "None" :!class /Script/Engine.KismetMaterialLibrary))
    (bind _output_get_2 (Variables|EasySnowSettings|SetDynamicMaterial _returnvalue_3))
    (Class|NiagaraComponent|SetVariableMaterial (Variables|Default|GetSnowBP) "NiagaraDebug_Mid" _output_get_2)
    (Rendering|Material|SetScalarParameterValue (Variables|EasySnowSettings|GetDynamicMaterial) "DebugToggleMaterial_Mid" _returnvalue :!class /Script/Engine.MaterialInstanceDynamic)
    (bind _returnvalue_4 (Rendering|Material|CreateDynamicMaterialInstance "/Game/EasySnow/Materials/Masters/M_niagaraSnow.M_niagaraSnow" "None" "None" :!class /Script/Engine.KismetMaterialLibrary))
    (bind _output_get_3 (Variables|EasySnowSettings|SetDynamicMaterial _returnvalue_4))
    (Class|NiagaraComponent|SetVariableMaterial (Variables|Default|GetSnowBP) "NiagaraDebug_Far" _output_get_3)
    (Rendering|Material|SetScalarParameterValue (Variables|EasySnowSettings|GetDynamicMaterial) "DebugToggleMaterial_Far" _returnvalue :!class /Script/Engine.MaterialInstanceDynamic)
    (else
      ;[1 1 1] Snowflake Material Variables
      (bind _returnvalue_5 (Rendering|Material|CreateDynamicMaterialInstance "/Game/EasySnow/Materials/Masters/M_niagaraSnow.M_niagaraSnow" "None" "None" :!class /Script/Engine.KismetMaterialLibrary))
      (bind _output_get_4 (Variables|EasySnowSettings|SetDynamicMaterial _returnvalue_5))
      (Class|NiagaraComponent|SetVariableMaterial _snowbp_16 "NiagaraDebug_Near" _output_get_4)
      (Class|NiagaraComponent|SetVariableMaterial _snowbp_16 "NiagaraDebug_Mid" _output_get_4)
      (Class|NiagaraComponent|SetVariableMaterial _snowbp_16 "NiagaraDebug_Mid" _output_get_4)
      (Rendering|Material|SetVectorParameterValue (Variables|EasySnowSettings|GetDynamicMaterial) "Base Color" (Variables|EasySnowSettings|SnowflakeMaterialAdjustments|GetbaseColor) :!class /Script/Engine.MaterialInstanceDynamic)
      (Rendering|Material|SetScalarParameterValue (Variables|EasySnowSettings|GetDynamicMaterial) "Roughness" (Variables|EasySnowSettings|SnowflakeMaterialAdjustments|Getroughness) :!class /Script/Engine.MaterialInstanceDynamic)
      (Rendering|Material|SetScalarParameterValue (Variables|EasySnowSettings|GetDynamicMaterial) "Normal Tiling" (Variables|EasySnowSettings|SnowflakeMaterialAdjustments|GetnormalTiling) :!class /Script/Engine.MaterialInstanceDynamic)
      (Rendering|Material|SetScalarParameterValue (Variables|EasySnowSettings|GetDynamicMaterial) "Normal Intensity" (Variables|EasySnowSettings|SnowflakeMaterialAdjustments|GetnormalIntensity) :!class /Script/Engine.MaterialInstanceDynamic)
      (Rendering|Material|SetScalarParameterValue (Variables|EasySnowSettings|GetDynamicMaterial) "Subsurface Intensity" (Variables|EasySnowSettings|SnowflakeMaterialAdjustments|GetsubsurfaceIntensity) :!class /Script/Engine.MaterialInstanceDynamic)
      (Rendering|Material|SetVectorParameterValue (Variables|EasySnowSettings|GetDynamicMaterial) "Subsurface Color" (Variables|EasySnowSettings|SnowflakeMaterialAdjustments|GetsubsurfaceColor) :!class /Script/Engine.MaterialInstanceDynamic)
      (Rendering|Material|SetVectorParameterValue (Variables|EasySnowSettings|GetDynamicMaterial) "snowEmissive" (Variables|EasySnowSettings|SnowflakeMaterialAdjustments|GetsnowEmissive) :!class /Script/Engine.MaterialInstanceDynamic)
      (Rendering|Material|SetScalarParameterValue (Variables|EasySnowSettings|GetDynamicMaterial) "Camera Fading Distance" (Variables|EasySnowSettings|SnowflakeMaterialAdjustments|GetcameraFadeDistance) :!class /Script/Engine.MaterialInstanceDynamic)
      ;[1 1 1] Sprite Material Variables
      (bind _returnvalue_6 (Rendering|Material|CreateDynamicMaterialInstance "/Game/EasySnow/Materials/Masters/M_niagaraSnowSprite.M_niagaraSnowSprite" "None" "None" :!class /Script/Engine.KismetMaterialLibrary))
      (bind _output_get_5 (Variables|EasySnowSettings|SetspriteDynamicMaterial _returnvalue_6))
      (Class|NiagaraComponent|SetVariableMaterial (Variables|Default|GetSnowBP) "NiagaraDebug_Far" _output_get_5)
      (Rendering|Material|SetVectorParameterValue (Variables|EasySnowSettings|GetspriteDynamicMaterial) "Base Color" (Variables|EasySnowSettings|SnowflakeMaterialAdjustments|GetbaseColor) :!class /Script/Engine.MaterialInstanceDynamic)
      (Rendering|Material|SetScalarParameterValue (Variables|EasySnowSettings|GetspriteDynamicMaterial) "Subsurface Intensity" (Variables|EasySnowSettings|SnowflakeMaterialAdjustments|GetsubsurfaceIntensity) :!class /Script/Engine.MaterialInstanceDynamic)
      (Rendering|Material|SetVectorParameterValue (Variables|EasySnowSettings|GetspriteDynamicMaterial) "Subsurface Color" (Variables|EasySnowSettings|SnowflakeMaterialAdjustments|GetsubsurfaceColor) :!class /Script/Engine.MaterialInstanceDynamic)
      (Rendering|Material|SetScalarParameterValue (Variables|EasySnowSettings|GetspriteDynamicMaterial) "AlphaMult" (Variables|EasySnowSettings|GetdistantParticleAlpha) :!class /Script/Engine.MaterialInstanceDynamic)
      (Rendering|Material|SetVectorParameterValue (Variables|EasySnowSettings|GetspriteDynamicMaterial) "snowEmissive" (Variables|EasySnowSettings|SnowflakeMaterialAdjustments|GetsnowEmissive) :!class /Script/Engine.MaterialInstanceDynamic)))
  ;[1 1 1] Drifts Material Variables
  (bind _returnvalue_7 (Rendering|Material|CreateDynamicMaterialInstance "/Game/EasySnow/Materials/Masters/M_niagaraDriftingSnow_01.M_niagaraDriftingSnow_01" "None" "None" :!class /Script/Engine.KismetMaterialLibrary))
  (bind _output_get_6 (Variables|EasySnowSettings|SetdriftsDynamicMaterial _returnvalue_7))
  (Class|NiagaraComponent|SetVariableMaterial (Variables|Default|GetSnowBP) "DriftsMaterial" _output_get_6)
  (Rendering|Material|SetVectorParameterValue (Variables|EasySnowSettings|GetdriftsDynamicMaterial) "driftsColor" (Variables|EasySnowSettings|Drifts|DriftMaterialAdjustments|GetdriftColor) :!class /Script/Engine.MaterialInstanceDynamic)
  (Rendering|Material|SetScalarParameterValue (Variables|EasySnowSettings|GetdriftsDynamicMaterial) "Fading Distance" (Variables|EasySnowSettings|Drifts|DriftMaterialAdjustments|GetGeometry%20Fading%20Distance) :!class /Script/Engine.MaterialInstanceDynamic)
  (Rendering|Material|SetVectorParameterValue (Variables|EasySnowSettings|GetdriftsDynamicMaterial) "driftsEmissive" (Variables|EasySnowSettings|Drifts|DriftMaterialAdjustments|GetdriftsEmissive) :!class /Script/Engine.MaterialInstanceDynamic)
  (Rendering|Material|SetScalarParameterValue (Variables|EasySnowSettings|GetdriftsDynamicMaterial) "driftsAnimationSpeed" (Variables|EasySnowSettings|Drifts|DriftMaterialAdjustments|GetdriftsTextureSpeed) :!class /Script/Engine.MaterialInstanceDynamic)
  (Rendering|Material|SetScalarParameterValue (Variables|EasySnowSettings|GetdriftsDynamicMaterial) "Drifts Camera Fading Distance" (Variables|EasySnowSettings|Drifts|DriftMaterialAdjustments|GetdriftsCameraFadeDistance) :!class /Script/Engine.MaterialInstanceDynamic)
  (Niagara|SetNiagaraVariable(Float) (Variables|Default|GetSnowBP) "distantParticleScale" (Variables|EasySnowSettings|GetdistantParticleSize%20-))
  (Niagara|SetNiagaraVariable(Float) (Variables|Default|GetSnowBP) "MidDetailSnowflakesMaxDistance" (Variables|EasySnowSettings|LODControl|GetMidDetailMaxDistance))
  (Niagara|SetNiagaraVariable(Float) (Variables|Default|GetSnowBP) "HighDetailSnowflakesMaxDistance" (Variables|EasySnowSettings|LODControl|GetHighDetailMaxDistance))
  (Niagara|SetNiagaraVariable(Bool) (Variables|Default|GetSnowBP) "Global Snow" (Variables|EasySnowSettings|GetCamera-Centric))
  (Class|NiagaraComponent|SetCustomTimeDilation (Variables|Default|GetSnowBP) (Variables|EasySnowSettings|GetcustomSpeed%20-))
  (Niagara|SetNiagaraVariable(Bool) (Variables|Default|GetSnowBP) "collision" (Variables|EasySnowSettings|Getcollision))
  (Niagara|SetNiagaraVariable(Float) (Variables|Default|GetSnowBP) "spawnRadius" (Variables|EasySnowSettings|GetspawnRadius))
  (Niagara|SetNiagaraVariable(Float) (Variables|Default|GetSnowBP) "driftsAdditionalDrag" (Variables|EasySnowSettings|Drifts|GetdriftsAdditionalDrag%20-))
  (Niagara|SetNiagaraVariable(Float) (Variables|Default|GetSnowBP) "spawnRadiusHeight" (Variables|EasySnowSettings|GetspawnRadiusHeight))
  (Niagara|SetNiagaraVariable(Float) (Variables|Default|GetSnowBP) "windDirection" (Variables|EasySnowSettings|Wind|GetwindDirection))
  (Niagara|SetNiagaraVariable(Float) (Variables|Default|GetSnowBP) "motionScaleDistantFlakes" (Variables|EasySnowSettings|GetdistantParticleMotionScale))
  (Rendering|Material|SetScalarParameterValue "/Game/EasySnow/System/MP_WF_WorldData.MP_WF_WorldData" "windDirection" (Variables|EasySnowSettings|Wind|GetwindDirection) :!class /Script/Engine.KismetMaterialLibrary)
  (Rendering|Material|SetScalarParameterValue "/Game/EasySnow/System/MP_WF_WorldData.MP_WF_WorldData" "windStrength" (Variables|EasySnowSettings|Wind|GetwindStrength%20-) :!class /Script/Engine.KismetMaterialLibrary)
  (Rendering|SetCastShadow (Variables|Default|GetSnowBP) (Variables|EasySnowSettings|GetcastShadow))
  (if (Variables|EasySnowSettings|WorldMaterialSettings|GetSet%20World%20Snow%20Material%20Settings)
    ;[1 1 1] World Material Snow Control
    (Rendering|Material|SetScalarParameterValue "/Game/EasySnow/System/MP_WF_WorldData.MP_WF_WorldData" "windBuildupOverride" (Variables|EasySnowSettings|WorldMaterialSettings|GetwindBuildupOverride) :!class /Script/Engine.KismetMaterialLibrary)
    (Rendering|Material|SetScalarParameterValue "/Game/EasySnow/System/MP_WF_WorldData.MP_WF_WorldData" "Snow Glimmering Intensity" (Variables|EasySnowSettings|WorldMaterialSettings|GetSnow%20Glimmer%20Intensity) :!class /Script/Engine.KismetMaterialLibrary)
    (Rendering|Material|SetScalarParameterValue "/Game/EasySnow/System/MP_WF_WorldData.MP_WF_WorldData" "Snow Displacement Multiplier" (Variables|EasySnowSettings|WorldMaterialSettings|GetWorld%20Snow%20Displacement%20Multiplier) :!class /Script/Engine.KismetMaterialLibrary)
    (Rendering|Material|SetScalarParameterValue "/Game/EasySnow/System/MP_WF_WorldData.MP_WF_WorldData" "Z Offset" (Variables|EasySnowSettings|WorldMaterialSettings|GetZ%20%20Offset) :!class /Script/Engine.KismetMaterialLibrary)
    (Rendering|Material|SetScalarParameterValue "/Game/EasySnow/System/MP_WF_WorldData.MP_WF_WorldData" "Transition Sharpness" (Variables|EasySnowSettings|WorldMaterialSettings|GetTransition%20Sharpness) :!class /Script/Engine.KismetMaterialLibrary)
    (Rendering|Material|SetScalarParameterValue "/Game/EasySnow/System/MP_WF_WorldData.MP_WF_WorldData" "Breakup Intensity" (Variables|EasySnowSettings|WorldMaterialSettings|GetbreakupIntensity) :!class /Script/Engine.KismetMaterialLibrary)
    (Rendering|Material|SetScalarParameterValue "/Game/EasySnow/System/MP_WF_WorldData.MP_WF_WorldData" "Breakup Texture Tiling" (Math|Conversions|ToFloat(Integer) (Class|KismetMathLibrary|ToInt64(Float) (Variables|EasySnowSettings|WorldMaterialSettings|GetbreakupTextureTiling))) :!class /Script/Engine.KismetMaterialLibrary)
    (Rendering|Material|SetScalarParameterValue "/Game/EasySnow/System/MP_WF_WorldData.MP_WF_WorldData" "Snow Fade Control" (Variables|EasySnowSettings|WorldMaterialSettings|GetsnowFadeControl) :!class /Script/Engine.KismetMaterialLibrary)
    (Rendering|Material|SetScalarParameterValue "/Game/EasySnow/System/MP_WF_WorldData.MP_WF_WorldData" "Snow Amount" (Variables|EasySnowSettings|WorldMaterialSettings|GetsnowAmount) :!class /Script/Engine.KismetMaterialLibrary))
  ;[1 1 1] Presets
  (bind _preset (Variables|EasySnowSettings|GetPreset) ; Getting Preset Data
    (:then
      (Niagara|SetNiagaraVariable(Float) _snowbp_4 "spawnRate" (Variables|/Game/EasySnow/System/Presets/BP_EasySnow_Presets.BP_EasySnow_Presets_C|GetspawnRate _preset))
      (Variables|EasySnowSettings|SetspawnRate%20- (Variables|/Game/EasySnow/System/Presets/BP_EasySnow_Presets.BP_EasySnow_Presets_C|GetspawnRate _preset))
      (Niagara|SetNiagaraVariable(Float) _snowbp_12 "windStrength" (Variables|/Game/EasySnow/System/Presets/BP_EasySnow_Presets.BP_EasySnow_Presets_C|GetwindStrength _preset))
      (Variables|EasySnowSettings|Wind|SetwindStrength%20- (Variables|/Game/EasySnow/System/Presets/BP_EasySnow_Presets.BP_EasySnow_Presets_C|GetwindStrength _preset))
      (Niagara|SetNiagaraVariable(Float) _snowbp_7 "snowLifetime" (Variables|/Game/EasySnow/System/Presets/BP_EasySnow_Presets.BP_EasySnow_Presets_C|GetsnowLifetime _preset))
      (Variables|EasySnowSettings|SetsnowLifetime%20- (Variables|/Game/EasySnow/System/Presets/BP_EasySnow_Presets.BP_EasySnow_Presets_C|GetsnowLifetime _preset))
      (Niagara|SetNiagaraVariable(Float) _snowbp_9 "flurriesMin" (Variables|/Game/EasySnow/System/Presets/BP_EasySnow_Presets.BP_EasySnow_Presets_C|GetairResistanceMin _preset))
      (Variables|EasySnowSettings|SetAir%20Resistance%20Min%20- (Variables|/Game/EasySnow/System/Presets/BP_EasySnow_Presets.BP_EasySnow_Presets_C|GetairResistanceMin _preset))
      (Niagara|SetNiagaraVariable(Float) _snowbp_11 "flurriesMax" (Variables|/Game/EasySnow/System/Presets/BP_EasySnow_Presets.BP_EasySnow_Presets_C|GetairResistanceMax _preset))
      (Variables|EasySnowSettings|SetAir%20Resistance%20Max%20- (Variables|/Game/EasySnow/System/Presets/BP_EasySnow_Presets.BP_EasySnow_Presets_C|GetairResistanceMax _preset))
      (Niagara|SetNiagaraVariable(Float) _snowbp_17 "snowChaos" (Variables|/Game/EasySnow/System/Presets/BP_EasySnow_Presets.BP_EasySnow_Presets_C|GetsnowChaos _preset))
      (Variables|EasySnowSettings|SetsnowChaos%20- (Variables|/Game/EasySnow/System/Presets/BP_EasySnow_Presets.BP_EasySnow_Presets_C|GetsnowChaos _preset))
      (Niagara|SetNiagaraVariable(Float) _snowbp_13 "driftsSpawnRate" (Variables|/Game/EasySnow/System/Presets/BP_EasySnow_Presets.BP_EasySnow_Presets_C|GetdriftingSnowAmount _preset))
      (Variables|EasySnowSettings|Drifts|SetDriftingSnowAmount%20- (Variables|/Game/EasySnow/System/Presets/BP_EasySnow_Presets.BP_EasySnow_Presets_C|GetdriftingSnowAmount _preset))
      (Niagara|SetNiagaraVariable(Float) _snowbp_10 "additionalDrag" (Variables|/Game/EasySnow/System/Presets/BP_EasySnow_Presets.BP_EasySnow_Presets_C|GetadditionalDrag _preset))
      (Variables|EasySnowSettings|SetadditionalDrag%20- (Variables|/Game/EasySnow/System/Presets/BP_EasySnow_Presets.BP_EasySnow_Presets_C|GetadditionalDrag _preset))
      (Niagara|SetNiagaraVariable(Bool) _snowbp_3 "driftsEnable" (Variables|/Game/EasySnow/System/Presets/BP_EasySnow_Presets.BP_EasySnow_Presets_C|GetdriftsEnable _preset))
      (Variables|EasySnowSettings|Drifts|SetdriftsEnable%20- (Variables|/Game/EasySnow/System/Presets/BP_EasySnow_Presets.BP_EasySnow_Presets_C|GetdriftsEnable _preset))
      (Niagara|SetNiagaraVariable(Float) _snowbp_8 "NearParticleSizeMin" (Variables|/Game/EasySnow/System/Presets/BP_EasySnow_Presets.BP_EasySnow_Presets_C|GetNearParticleSizeMin _preset))
      (Variables|EasySnowSettings|SetNearParticleSizeMin%20- (Variables|/Game/EasySnow/System/Presets/BP_EasySnow_Presets.BP_EasySnow_Presets_C|GetNearParticleSizeMin _preset))
      (Niagara|SetNiagaraVariable(Float) _snowbp_2 "NearParticleSizeMax" (Variables|/Game/EasySnow/System/Presets/BP_EasySnow_Presets.BP_EasySnow_Presets_C|GetNearParticleSizeMax _preset))
      (Variables|EasySnowSettings|SetNearParticleSizeMax%20- (Variables|/Game/EasySnow/System/Presets/BP_EasySnow_Presets.BP_EasySnow_Presets_C|GetNearParticleSizeMax _preset))
      (Niagara|SetNiagaraVariable(Float) _snowbp_14 "distantParticleScale" (Variables|/Game/EasySnow/System/Presets/BP_EasySnow_Presets.BP_EasySnow_Presets_C|GetdistantParticleScale _preset))
      (Variables|EasySnowSettings|SetdistantParticleSize%20- (Variables|/Game/EasySnow/System/Presets/BP_EasySnow_Presets.BP_EasySnow_Presets_C|GetdistantParticleScale _preset))
      (Niagara|SetNiagaraVariable(Float) _snowbp_15 "turbulenceIntensity" (Variables|/Game/EasySnow/System/Presets/BP_EasySnow_Presets.BP_EasySnow_Presets_C|GetturbulenceIntensity _preset))
      (Variables|EasySnowSettings|Wind|Turbulence|SetturbulenceIntensity%20- (Variables|/Game/EasySnow/System/Presets/BP_EasySnow_Presets.BP_EasySnow_Presets_C|GetturbulenceIntensity _preset))
      (Niagara|SetNiagaraVariable(Float) _snowbp_6 "turbulenceFrequency" (Variables|/Game/EasySnow/System/Presets/BP_EasySnow_Presets.BP_EasySnow_Presets_C|GetturbulenceFrequency _preset))
      (Variables|EasySnowSettings|Wind|Turbulence|SetturbulenceFrequency%20- (Variables|/Game/EasySnow/System/Presets/BP_EasySnow_Presets.BP_EasySnow_Presets_C|GetturbulenceFrequency _preset))
      (Niagara|SetNiagaraVariable(Bool) _snowbp_5 "toggleGravity" (Variables|/Game/EasySnow/System/Presets/BP_EasySnow_Presets.BP_EasySnow_Presets_C|GettoggleGravity _preset))
      (Variables|EasySnowSettings|SettoggleGravity%20- (Variables|/Game/EasySnow/System/Presets/BP_EasySnow_Presets.BP_EasySnow_Presets_C|GettoggleGravity _preset))
      (Niagara|SetNiagaraVariable(Bool) _snowbp "toggleDriftGravity" (Variables|/Game/EasySnow/System/Presets/BP_EasySnow_Presets.BP_EasySnow_Presets_C|GettoggleDriftGravity _preset))
      (Variables|EasySnowSettings|Drifts|SettoggleDriftGravity%20- (Variables|/Game/EasySnow/System/Presets/BP_EasySnow_Presets.BP_EasySnow_Presets_C|GettoggleDriftGravity _preset))
      (Niagara|SetNiagaraVariable(Float) (Variables|Default|GetSnowBP) "driftsSizeMin" (Variables|/Game/EasySnow/System/Presets/BP_EasySnow_Presets.BP_EasySnow_Presets_C|GetdriftsSizeMin _preset))
      (Variables|EasySnowSettings|Drifts|SetdriftsSizeMin%20- (Variables|/Game/EasySnow/System/Presets/BP_EasySnow_Presets.BP_EasySnow_Presets_C|GetdriftsSizeMin _preset))
      (Niagara|SetNiagaraVariable(Float) (Variables|Default|GetSnowBP) "driftsSizeMax" (Variables|/Game/EasySnow/System/Presets/BP_EasySnow_Presets.BP_EasySnow_Presets_C|GetdriftsSizeMax _preset))
      (Variables|EasySnowSettings|Drifts|SetdriftsSizeMax%20- (Variables|/Game/EasySnow/System/Presets/BP_EasySnow_Presets.BP_EasySnow_Presets_C|GetdriftsSizeMax _preset))
      (Rendering|Material|SetScalarParameterValue (Variables|EasySnowSettings|GetdriftsDynamicMaterial) "driftOpacity" (Variables|/Game/EasySnow/System/Presets/BP_EasySnow_Presets.BP_EasySnow_Presets_C|GetdriftsOpacity _preset) :!class /Script/Engine.MaterialInstanceDynamic)
      (Variables|EasySnowSettings|Drifts|SetdriftOpacity%20- (Variables|/Game/EasySnow/System/Presets/BP_EasySnow_Presets.BP_EasySnow_Presets_C|GetdriftsOpacity _preset))
      (Niagara|SetNiagaraVariable(Float) (Variables|Default|GetSnowBP) "windUpdraftStrength" (Variables|/Game/EasySnow/System/Presets/BP_EasySnow_Presets.BP_EasySnow_Presets_C|GetwindUpdraftStrength _preset))
      (Variables|EasySnowSettings|Wind|SetwindUpdraftStrength%20- (Variables|/Game/EasySnow/System/Presets/BP_EasySnow_Presets.BP_EasySnow_Presets_C|GetwindUpdraftStrength _preset))
      (Class|NiagaraComponent|SetCustomTimeDilation (Variables|Default|GetSnowBP) (Variables|/Game/EasySnow/System/Presets/BP_EasySnow_Presets.BP_EasySnow_Presets_C|GetcustomSpeed _preset))
      (Variables|EasySnowSettings|SetcustomSpeed%20- (Variables|/Game/EasySnow/System/Presets/BP_EasySnow_Presets.BP_EasySnow_Presets_C|GetcustomSpeed _preset)))
    (:else
      (Niagara|SetNiagaraVariable(Float) _snowbp_4 "spawnRate" (Variables|EasySnowSettings|GetspawnRate%20-))
      (Niagara|SetNiagaraVariable(Float) _snowbp_12 "windStrength" (Variables|EasySnowSettings|Wind|GetwindStrength%20-))
      (Niagara|SetNiagaraVariable(Float) _snowbp_7 "snowLifetime" (Variables|EasySnowSettings|GetsnowLifetime%20-))
      (Niagara|SetNiagaraVariable(Float) _snowbp_9 "flurriesMin" (Variables|EasySnowSettings|GetAir%20Resistance%20Min%20-))
      (Niagara|SetNiagaraVariable(Float) _snowbp_11 "flurriesMax" (Variables|EasySnowSettings|GetAir%20Resistance%20Max%20-))
      (Niagara|SetNiagaraVariable(Float) _snowbp_17 "snowChaos" (Variables|EasySnowSettings|GetsnowChaos%20-))
      (Niagara|SetNiagaraVariable(Float) _snowbp_13 "driftsSpawnRate" (Variables|EasySnowSettings|Drifts|GetDriftingSnowAmount%20-))
      (Niagara|SetNiagaraVariable(Float) _snowbp_10 "additionalDrag" (Variables|EasySnowSettings|GetadditionalDrag%20-))
      (Niagara|SetNiagaraVariable(Bool) _snowbp_3 "driftsEnable" (Variables|EasySnowSettings|Drifts|GetdriftsEnable%20-))
      (Niagara|SetNiagaraVariable(Float) _snowbp_8 "NearParticleSizeMin" (Variables|EasySnowSettings|GetNearParticleSizeMin%20-))
      (Niagara|SetNiagaraVariable(Float) _snowbp_2 "NearParticleSizeMax" (Variables|EasySnowSettings|GetNearParticleSizeMax%20-))
      (Niagara|SetNiagaraVariable(Float) _snowbp_14 "distantParticleScale" (Variables|EasySnowSettings|GetdistantParticleSize%20-))
      (Niagara|SetNiagaraVariable(Float) _snowbp_15 "turbulenceIntensity" (Variables|EasySnowSettings|Wind|Turbulence|GetturbulenceIntensity%20-))
      (Niagara|SetNiagaraVariable(Float) _snowbp_6 "turbulenceFrequency" (Variables|EasySnowSettings|Wind|Turbulence|GetturbulenceFrequency%20-))
      (Niagara|SetNiagaraVariable(Bool) _snowbp_5 "toggleGravity" (Variables|EasySnowSettings|GettoggleGravity%20-))
      (Niagara|SetNiagaraVariable(Bool) _snowbp "toggleDriftGravity" (Variables|EasySnowSettings|Drifts|GettoggleDriftGravity%20-))
      (Niagara|SetNiagaraVariable(Float) (Variables|Default|GetSnowBP) "driftsSizeMin" (Variables|EasySnowSettings|Drifts|GetdriftsSizeMin%20-))
      (Niagara|SetNiagaraVariable(Float) (Variables|Default|GetSnowBP) "driftsSizeMax" (Variables|EasySnowSettings|Drifts|GetdriftsSizeMax%20-))
      (Rendering|Material|SetScalarParameterValue (Variables|EasySnowSettings|GetdriftsDynamicMaterial) "driftOpacity" (Variables|EasySnowSettings|Drifts|GetdriftOpacity%20-) :!class /Script/Engine.MaterialInstanceDynamic)
      (Niagara|SetNiagaraVariable(Float) (Variables|Default|GetSnowBP) "windUpdraftStrength" (Variables|EasySnowSettings|Wind|GetwindUpdraftStrength%20-))
      (Class|NiagaraComponent|SetCustomTimeDilation (Variables|Default|GetSnowBP) (Variables|EasySnowSettings|GetcustomSpeed%20-)))))

(fn ExtractVariablesfromPreset
  (params (spawnRate :type Float%20%28double-precision%29) (Preset :type Data%20Asset%20Link%20Object%20Reference)))