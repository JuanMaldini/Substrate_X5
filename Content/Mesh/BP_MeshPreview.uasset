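; BP_MeshPreview is a display actor that previews a static mesh and material with two 3D text labels.
; Its construction script applies the StaticMesh and Material (slot 0) variables to the Sphere component.
; It fills the labels from Text1, converted to uppercase, and Text2, then halves the relative scale of both.
; The event graph holds only disabled stub events, so it adds no runtime logic.
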(event EventBeginPlay)

(event Collision|EventActorBeginOverlap
  (params (OtherActor :type Actor%20Object%20Reference)))

(event EventTick
  (params (DeltaSeconds :type Float%20%28single-precision%29)))

(fn ConstructionScript
  (bind _returnvalue (Math|Conversions|ToVector(Float) 0.5))
  (bind _text3d1 (Variables|Default|Gettext3d1))
  (bind _text3d (Variables|Default|Gettext3d))
  (bind _returnvalue_2 (Transformation|GetRelativeTransform _text3d1))
  (bind _returnvalue_3 (Transformation|GetRelativeTransform _text3d))
  (Class|Text3DComponent|SetText (Variables|Default|Gettext3d) (Class|KismetTextLibrary|TexttoUpper (Variables|Default|GetText%20%201)))
  (Rendering|Material|SetMaterial (Variables|Default|GetSphere) 0 (Variables|Default|GetMaterial))
  (Class|Text3DComponent|SetText (Variables|Default|Gettext3d1) (Variables|Default|GetText%202))
  (Components|StaticMesh|SetStaticMesh (Variables|Default|GetSphere) (Variables|Default|GetStatic%20Mesh))
  (Transformation|SetRelativeTransform _text3d1 (Math|Transform|MakeTransform (.location _returnvalue_2) (.rotation _returnvalue_2) (* (.scale _returnvalue_2) _returnvalue)) false false)
  (Transformation|SetRelativeTransform _text3d (Math|Transform|MakeTransform (.location _returnvalue_3) (.rotation _returnvalue_3) (* (.scale _returnvalue_3) _returnvalue)) false false))